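; BP_StoneTool is an editor placement tool that scatters randomized static meshes, presumably stones or gems, around the actor.
; Its construction script adds QtdGems mesh components, each with a random relative location and non-uniform scale drawn from per-axis min/max ranges.
; Each component gets a random mesh from MeshArray.
; Rotation is not randomized, the random stream is unseeded, and the event graph is empty.
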(event EventBeginPlay)

(event Collision|EventActorBeginOverlap
  (params (OtherActor :type Actor%20Object%20Reference)))

(event EventTick
  (params (DeltaSeconds :type Float%20%28single-precision%29)))

(fn ConstructionScript
  (bind _scale_y (Variables|GemsConfig|GetScale%20Y))
  (bind _scale_z (Variables|GemsConfig|GetScale%20Z))
  (bind _mesharray (Variables|Default|GetMeshArray))
  (bind _transform_x (Variables|GemsConfig|GetTransform%20X))
  (bind _transform_y (Variables|GemsConfig|GetTransform%20Y))
  (bind _transform_z (Variables|GemsConfig|GetTransform%20Z))
  (bind _scale_x (Variables|GemsConfig|GetScale%20X))
  (for _index (range 1 (Variables|GemsConfig|GetQtdGems))
    (bind _returnvalue (AddComponent|AddStaticMeshComponent false (Math|Transform|MakeTransform (Math|Vector|MakeVector (Math|Random|RandomFloatinRange (.x _transform_x) (.y _transform_x)) (Math|Random|RandomFloatinRange (.x _transform_y) (.y _transform_y)) (Math|Random|RandomFloatinRange (.x _transform_z) (.y _transform_z))) "0, 0, 0" (Math|Vector|MakeVector (Math|Random|RandomFloatinRange (.x _scale_x) (.y _scale_x)) (Math|Random|RandomFloatinRange (.x _scale_y) (.y _scale_y)) (Math|Random|RandomFloatinRange (.x _scale_z) (.y _scale_z))))))
    (Components|StaticMesh|SetStaticMesh _returnvalue (Utilities|Array|Get(acopy) _mesharray (Math|Random|RandomIntegerinRange 0 (Utilities|Array|LastIndex _mesharray))))))