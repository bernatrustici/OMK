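; Procedural modular room builder that assembles floor, four walls and roof in the Construction Script, each toggleable and sized by SizeX/Y/Z.
; Nested loops add Static Mesh Components on a grid, picking meshes by index from MeshVariationList.
; With Windowned on, SetVariationWindow swaps in a per-side variation mesh on the bottom wall row.
; It reloads its helpers every call, discarding CountCtrl's step and quantity updates, so only one step matches per wall.
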(event EventBeginPlay)

(event Collision|EventActorBeginOverlap
  (params (OtherActor :type Actor%20Object%20Reference)))

(event EventTick
  (params (DeltaSeconds :type Float%20%28single-precision%29)))

(fn ConstructionScript
  (bind _size_z (Variables|Transform|GetSize%20Z))
  (bind _transform_z (Variables|Transform|GetTransform%20Z))
  (bind _transform_y_r (Variables|TransformWallRight|GetTransform%20Y%20R))
  (bind _transform_z_2 (Variables|Transform|GetTransform%20Z))
  (bind _transform_x_b (Variables|TransformWallBack|GetTransform%20X%20B))
  (bind _transform_x_f (Variables|Transformwallfront|GetTransform%20X%20F))
  (bind _size_x (Variables|Transform|GetSize%20X))
  (bind _transform_x (Variables|Transform|GetTransform%20X))
  (bind _transform_y (Variables|Transform|GetTransform%20Y))
  (bind _size_y (Variables|Transform|GetSize%20Y))
  (bind _size_x_2 (Variables|Transform|GetSize%20X))
  (bind _size_y_2 (Variables|Transform|GetSize%20Y))
  (bind _returnvalue (Math|Conversions|ToFloat(Integer) _transform_y_r))
  (bind _returnvalue_2 (Math|Conversions|ToFloat(Integer) _transform_x_b))
  (bind _returnvalue_3 (Math|Conversions|ToFloat(Integer) _transform_x_f))
  (bind _returnvalue_4 (* _size_z _transform_z))
  (bind _returnvalue_5 (* _size_y _transform_y))
  (bind _returnvalue_6 (* _size_x _transform_x))
  (bind _returnvalue_7 (Math|Conversions|ToFloat(Integer) _returnvalue_6))
  (bind _returnvalue_8 (Math|Conversions|ToFloat(Integer) _returnvalue_5))
  (bind _returnvalue_9 (+ _transform_z_2 _returnvalue_4))
  (bind _returnvalue_10 (Math|Conversions|ToFloat(Integer) _returnvalue_9))
  (bind _returnvalue_11 (+ _returnvalue _returnvalue_8))
  (bind _returnvalue_12 (+ _returnvalue_3 _returnvalue_7))
  (if (Variables|Transform|GetFloor)
    ;[1 1 1] x
    (for _index (range 0 _size_x_2)
      (bind _returnvalue_13 (AddComponent|AddStaticMeshComponent false))
      (bind _newparam (CallFunction|GetMeshfromArray (Variables|Transform|GetFloor%20Mesh%20Index)))
      (Components|StaticMesh|SetStaticMesh _returnvalue_13 _newparam)
      (Transformation|SetRelativeTransform _returnvalue_13 (Math|Transform|MakeTransform (Math|Vector|MakeVector (Math|Conversions|ToFloat(Integer) (* _index (Variables|Transform|GetTransform%20X))) 0.0 0.0) "0, 0, 0" "1.000000,1.000000,1.000000") false false)
      ;[1 1 1] y
      (for _index_2 (range 1 _size_y_2)
        (bind _returnvalue_14 (AddComponent|AddStaticMeshComponent false))
        (bind _newparam_2 (CallFunction|GetMeshfromArray (Variables|Transform|GetFloor%20Mesh%20Index)))
        (Components|StaticMesh|SetStaticMesh _returnvalue_14 _newparam_2)
        (Transformation|SetRelativeTransform _returnvalue_14 (Math|Transform|MakeTransform (Math|Vector|MakeVector (Math|Conversions|ToFloat(Integer) (* _index (Variables|Transform|GetTransform%20X))) (Math|Conversions|ToFloat(Integer) (* _index_2 (Variables|Transform|GetTransform%20Y))) 0.0) "0, 0, 0" "1.000000,1.000000,1.000000") false false))))
  (if (Variables|Transform|GetLeft%20Wall)
    (Variables|WindowConfig|SetMeshCount 0)
    ;[1 1 1] wall left
    (for _index_3 (range 0 _size_x_2)
      (bind _returnvalue_15 (AddComponent|AddStaticMeshComponent false))
      (bind (_meshindex _qtdvar _stepsvar) (CallFunction|SetVariationWindow 9))
      (bind _newparam_3 (CallFunction|GetMeshfromArray _meshindex))
      (Components|StaticMesh|SetStaticMesh _returnvalue_15 _newparam_3)
      (Transformation|SetRelativeTransform _returnvalue_15 (Math|Transform|MakeTransform (Math|Vector|MakeVector (Math|Conversions|ToFloat(Integer) (* _index_3 (Variables|TransformWallLeft|GetTransform%20X%20L))) (Math|Conversions|ToFloat(Integer) (Variables|TransformWallLeft|GetTransform%20Y%20L)) (Math|Conversions|ToFloat(Integer) (Variables|TransformWallLeft|GetTransform%20Z%20L))) "0, 0, 0" "1.000000,1.000000,1.000000") false false)
      (CallFunction|CountCtrl _qtdvar _stepsvar)
      ;[1 1 1] wall left
      (for _index_4 (range 1 (Variables|Transform|GetSize%20Z))
        (bind _returnvalue_16 (AddComponent|AddStaticMeshComponent false))
        (bind _newparam_4 (CallFunction|GetMeshfromArray (Variables|TransformWallLeft|GetZ%20Mesh%20Index%20L)))
        (Components|StaticMesh|SetStaticMesh _returnvalue_16 _newparam_4)
        (Transformation|SetRelativeTransform _returnvalue_16 (Math|Transform|MakeTransform (Math|Vector|MakeVector (Math|Conversions|ToFloat(Integer) (* _index_3 (Variables|TransformWallLeft|GetTransform%20X%20L))) (Math|Conversions|ToFloat(Integer) (Variables|TransformWallLeft|GetTransform%20Y%20L)) (+ (Variables|TransformWallLeft|GetTransform%20Z%20L) (Math|Conversions|ToFloat(Integer) (* _index_4 (Variables|Transform|GetTransform%20Z))))) "0, 0, 0" "1.000000,1.000000,1.000000") false false))))
  (if (Variables|Transform|GetRight%20Wall)
    (Variables|WindowConfig|SetMeshCount 0)
    ;[1 1 1] wall right
    (for _index_5 (range 0 _size_x_2)
      (bind _returnvalue_17 (AddComponent|AddStaticMeshComponent false))
      (bind (_meshindex_2 _qtdvar_2 _stepsvar_2) (CallFunction|SetVariationWindow 3))
      (bind _newparam_5 (CallFunction|GetMeshfromArray _meshindex_2))
      (Components|StaticMesh|SetStaticMesh _returnvalue_17 _newparam_5)
      (Transformation|SetRelativeTransform _returnvalue_17 (Math|Transform|MakeTransform (Math|Vector|MakeVector (Math|Conversions|ToFloat(Integer) (* _index_5 (Variables|TransformWallRight|GetTransform%20X%20R))) _returnvalue_11 (Math|Conversions|ToFloat(Integer) (Variables|TransformWallRight|GetTransform%20Z%20R))) "0, 0, 0" "1.000000,1.000000,1.000000") false false)
      (CallFunction|CountCtrl _qtdvar_2 _stepsvar_2)
      ;[1 1 1] wall right
      (for _index_6 (range 1 (Variables|Transform|GetSize%20Z))
        (bind _returnvalue_18 (AddComponent|AddStaticMeshComponent false))
        (bind _newparam_6 (CallFunction|GetMeshfromArray (Variables|TransformWallRight|GetZ%20Mesh%20Index%20R)))
        (Components|StaticMesh|SetStaticMesh _returnvalue_18 _newparam_6)
        (Transformation|SetRelativeTransform _returnvalue_18 (Math|Transform|MakeTransform (Math|Vector|MakeVector (Math|Conversions|ToFloat(Integer) (* _index_5 (Variables|TransformWallRight|GetTransform%20X%20R))) _returnvalue_11 (+ (Variables|TransformWallLeft|GetTransform%20Z%20L) (Math|Conversions|ToFloat(Integer) (* _index_6 (Variables|Transform|GetTransform%20Z))))) "0, 0, 0" "1.000000,1.000000,1.000000") false false))))
  (if (Variables|Transform|GetBack%20Wall)
    (Variables|WindowConfig|SetMeshCount 0)
    ;[1 1 1] wall back
    (for _index_7 (range 0 _size_y_2)
      (bind _returnvalue_19 (AddComponent|AddStaticMeshComponent false))
      (bind (_meshindex_3 _qtdvar_3 _stepsvar_3) (CallFunction|SetVariationWindow 6))
      (bind _newparam_7 (CallFunction|GetMeshfromArray _meshindex_3))
      (Components|StaticMesh|SetStaticMesh _returnvalue_19 _newparam_7)
      (Transformation|SetRelativeTransform _returnvalue_19 (Math|Transform|MakeTransform (Math|Vector|MakeVector _returnvalue_2 (Math|Conversions|ToFloat(Integer) (* _index_7 (Variables|TransformWallBack|GetTransform%20Y%20B))) (Math|Conversions|ToFloat(Integer) (Variables|TransformWallBack|GetTransform%20Z%20B))) "0.000000,90.000000,0.000000" "1.000000,1.000000,1.000000") false false)
      (CallFunction|CountCtrl _qtdvar_3 _stepsvar_3)
      ;[1 1 1] wall back
      (for _index_8 (range 1 (Variables|Transform|GetSize%20Z))
        (bind _returnvalue_20 (AddComponent|AddStaticMeshComponent false))
        (bind _newparam_8 (CallFunction|GetMeshfromArray (Variables|TransformWallBack|GetZ%20Mesh%20Index%20B)))
        (Components|StaticMesh|SetStaticMesh _returnvalue_20 _newparam_8)
        (Transformation|SetRelativeTransform _returnvalue_20 (Math|Transform|MakeTransform (Math|Vector|MakeVector _returnvalue_2 (Math|Conversions|ToFloat(Integer) (* _index_7 (Variables|TransformWallBack|GetTransform%20Y%20B))) (+ (Variables|TransformWallBack|GetTransform%20Z%20B) (Math|Conversions|ToFloat(Integer) (* _index_8 (Variables|Transform|GetTransform%20Z))))) "0.000000,90.000000,0.000000" "1.000000,1.000000,1.000000") false false))))
  (if (Variables|Transform|GetFront%20Wall)
    (Variables|WindowConfig|SetMeshCount 0)
    ;[1 1 1] wall front
    (for _index_9 (range 0 _size_y_2)
      (bind _returnvalue_21 (AddComponent|AddStaticMeshComponent false))
      (bind (_meshindex_4 _qtdvar_4 _stepsvar_4) (CallFunction|SetVariationWindow 12))
      (bind _newparam_9 (CallFunction|GetMeshfromArray _meshindex_4))
      (Components|StaticMesh|SetStaticMesh _returnvalue_21 _newparam_9)
      (Transformation|SetRelativeTransform _returnvalue_21 (Math|Transform|MakeTransform (Math|Vector|MakeVector _returnvalue_12 (Math|Conversions|ToFloat(Integer) (* _index_9 (Variables|Transformwallfront|GetTransform%20Y%20F))) (Math|Conversions|ToFloat(Integer) (Variables|Transformwallfront|GetTransform%20Z%20F))) "0.000000,90.000000,0.000000" "1.000000,1.000000,1.000000") false false)
      (CallFunction|CountCtrl _qtdvar_4 _stepsvar_4)
      ;[1 1 1] wall front
      (for _index_10 (range 1 (Variables|Transform|GetSize%20Z))
        (bind _returnvalue_22 (AddComponent|AddStaticMeshComponent false))
        (bind _newparam_10 (CallFunction|GetMeshfromArray (Variables|Transformwallfront|GetZ%20Mesh%20Index%20F)))
        (Components|StaticMesh|SetStaticMesh _returnvalue_22 _newparam_10)
        (Transformation|SetRelativeTransform _returnvalue_22 (Math|Transform|MakeTransform (Math|Vector|MakeVector _returnvalue_12 (Math|Conversions|ToFloat(Integer) (* _index_9 (Variables|Transformwallfront|GetTransform%20Y%20F))) (+ (Variables|Transformwallfront|GetTransform%20Z%20F) (Math|Conversions|ToFloat(Integer) (* _index_10 (Variables|Transform|GetTransform%20Z))))) "0.000000,90.000000,0.000000" "1.000000,1.000000,1.000000") false false))))
  (if (Variables|Transform|GetRoof)
    ;[1 1 1] Roof
    (for _index_11 (range 0 (Variables|Transform|GetSize%20X))
      (bind _returnvalue_23 (AddComponent|AddStaticMeshComponent false))
      (bind _newparam_11 (CallFunction|GetMeshfromArray (Variables|Transform|GetRoof%20Mesh%20Index)))
      (Components|StaticMesh|SetStaticMesh _returnvalue_23 _newparam_11)
      (Transformation|SetRelativeTransform _returnvalue_23 (Math|Transform|MakeTransform (Math|Vector|MakeVector (Math|Conversions|ToFloat(Integer) (* _index_11 (Variables|Transform|GetTransform%20X))) 0.0 _returnvalue_10) "0, 0, 0" "1.000000,1.000000,1.000000") false false)
      ;[1 1 1] Roof
      (for _index_12 (range 1 (Variables|Transform|GetSize%20Y))
        (bind _returnvalue_24 (AddComponent|AddStaticMeshComponent false))
        (bind _newparam_12 (CallFunction|GetMeshfromArray (Variables|Transform|GetRoof%20Mesh%20Index)))
        (Components|StaticMesh|SetStaticMesh _returnvalue_24 _newparam_12)
        (Transformation|SetRelativeTransform _returnvalue_24 (Math|Transform|MakeTransform (Math|Vector|MakeVector (Math|Conversions|ToFloat(Integer) (* _index_11 (Variables|Transform|GetTransform%20X))) (Math|Conversions|ToFloat(Integer) (* _index_12 (Variables|Transform|GetTransform%20Y))) _returnvalue_10) "0, 0, 0" "1.000000,1.000000,1.000000") false false)))))

(fn GetMeshfromArray
  (params (MeshIndex :type Integer))
  (bind _output_get (Variables|WindowConfig|SetMeshResult (Utilities|Array|Get(acopy) (Variables|Transform|GetMeshVariationList) MeshIndex)))
  (return _output_get))

(fn SetVariationWindow
  (params (SideWall :type Integer))
  (bind _step_var_l (Variables|TransformWallLeft|GetStep%20Var%20L))
  (bind _step_var_r (Variables|TransformWallRight|GetStep%20Var%20R))
  (bind _step_var_b (Variables|TransformWallBack|GetStep%20Var%20B))
  (bind _step_var_f (Variables|Transformwallfront|GetStep%20Var%20F))
  (bind _size_x (Variables|Transform|GetSize%20X))
  (bind _size_y (Variables|Transform|GetSize%20Y))
  ;[1 1 1] CheckCardinalOrientation
  (if (== SideWall 9)
    (Variables|WindowConfig|SetMeshHelper (Variables|Transform|GetMesh%20Var%20Index%20L))
    (Variables|WindowConfig|SetMeshHelper2 (Variables|Transform|GetMesh%20Index%20L))
    (Variables|WindowConfig|SetQtd%20Var%20Helper (Variables|TransformWallLeft|GetQtd%20Var%20Mesh%20L))
    (Variables|WindowConfig|SetVar%20Steps%20Helper _step_var_l)
    (Variables|WindowConfig|SetVar%20Steps%20Helper2 _step_var_l)
    (Variables|WindowConfig|SetAxisHelper _size_x)
    (if (Variables|WindowConfig|GetWindowned) :!label _label
      ;[1 1 1] Select Mesh
      (if (>= (Variables|WindowConfig|GetAxisHelper) (Variables|WindowConfig|GetMeshCount))
        (if (== (+ (Variables|WindowConfig|GetMeshCount) 1) (Variables|WindowConfig|GetVar%20Steps%20Helper))
          (if (> (Variables|WindowConfig|GetQtd%20Var%20Helper) 0)
            (return (Variables|WindowConfig|GetMeshHelper) (> (Variables|WindowConfig|GetQtd%20Var%20Helper) 0) (== (+ (Variables|WindowConfig|GetMeshCount) 1) (Variables|WindowConfig|GetVar%20Steps%20Helper)))
            (else
              (return (Variables|WindowConfig|GetMeshHelper2) (> (Variables|WindowConfig|GetQtd%20Var%20Helper) 0) (== (+ (Variables|WindowConfig|GetMeshCount) 1) (Variables|WindowConfig|GetVar%20Steps%20Helper)))))
          (else
            (return (Variables|WindowConfig|GetMeshHelper2) (> (Variables|WindowConfig|GetQtd%20Var%20Helper) 0) (== (+ (Variables|WindowConfig|GetMeshCount) 1) (Variables|WindowConfig|GetVar%20Steps%20Helper)))))
        (else
          (return (Variables|WindowConfig|GetMeshHelper2) false false)))
      (else
        (return (Variables|WindowConfig|GetMeshHelper2) false false)))
    (elif (== SideWall 3)
      (Variables|WindowConfig|SetMeshHelper (Variables|Transform|GetMesh%20Var%20Index%20R))
      (Variables|WindowConfig|SetMeshHelper2 (Variables|Transform|GetMesh%20Index%20R))
      (Variables|WindowConfig|SetQtd%20Var%20Helper (Variables|TransformWallRight|GetQtd%20Var%20Mesh%20R))
      (Variables|WindowConfig|SetVar%20Steps%20Helper _step_var_r)
      (Variables|WindowConfig|SetVar%20Steps%20Helper2 _step_var_r)
      (Variables|WindowConfig|SetAxisHelper _size_x)
      (goto _label)
      (elif (== SideWall 6)
        (Variables|WindowConfig|SetMeshHelper (Variables|Transform|GetMesh%20Var%20Index%20B))
        (Variables|WindowConfig|SetMeshHelper2 (Variables|Transform|GetMesh%20Index%20B))
        (Variables|WindowConfig|SetQtd%20Var%20Helper (Variables|TransformWallBack|GetQtd%20Var%20Mesh%20B))
        (Variables|WindowConfig|SetVar%20Steps%20Helper _step_var_b)
        (Variables|WindowConfig|SetVar%20Steps%20Helper2 _step_var_b)
        (Variables|WindowConfig|SetAxisHelper _size_y)
        (goto _label)
        (elif (== SideWall 12)
          (Variables|WindowConfig|SetMeshHelper (Variables|Transform|GetMesh%20Var%20Index%20F))
          (Variables|WindowConfig|SetMeshHelper2 (Variables|Transform|GetMesh%20Index%20F))
          (Variables|WindowConfig|SetQtd%20Var%20Helper (Variables|Transformwallfront|GetQtd%20Var%20Mesh%20F))
          (Variables|WindowConfig|SetVar%20Steps%20Helper _step_var_f)
          (Variables|WindowConfig|SetVar%20Steps%20Helper2 _step_var_f)
          (Variables|WindowConfig|SetAxisHelper _size_y)
          (goto _label))))))

(fn CountCtrl
  (params (QtdVar :type Boolean) (StepsVar :type Boolean))
  (if StepsVar
    (Variables|WindowConfig|SetVar%20Steps%20Helper (+ (Variables|WindowConfig|GetVar%20Steps%20Helper) (Variables|WindowConfig|GetVar%20Steps%20Helper2))))
  (if QtdVar
    (bind _result (Math|Integer|DecrementInt (Variables|WindowConfig|GetQtd%20Var%20Helper))
      (:%20%20
        (Variables|WindowConfig|SetQtd%20Var%20Helper _result))))
  (bind _result_2 (Math|Integer|IncrementInt (Variables|WindowConfig|GetMeshCount))
    (:%20%20
      (Variables|WindowConfig|SetMeshCount _result_2))))

(fn SetVariationWindow2
  (params (SideWall :type Integer))
  (bind _qtd_var_mesh_l (Variables|TransformWallLeft|GetQtd%20Var%20Mesh%20L))
  (bind _returnvalue (> _qtd_var_mesh_l 0))
  (if (>= (+ (Variables|Transform|GetSize%20X) 10) (Variables|WindowConfig|GetMeshCount))
    (if _returnvalue
      (CallFunction|CountCtrl _returnvalue (== (Variables|WindowConfig|GetMeshCount) (Variables|TransformWallLeft|GetStep%20Var%20L)))
      (return (Variables|WindowConfig|GetMeshHelper)))))